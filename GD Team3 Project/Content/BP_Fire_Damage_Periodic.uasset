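; Fire hazard actor that damages any BP_MechCharacter entering its collision component and destroys itself ten seconds after Spawned_Fire is called.
; Begin overlap calls InFlame, shows the character's OnFire component and subtracts PlayerHealth directly in a Delay loop gated by one shared PlayerInRadius flag.
; Once that flag clears, a few lingering damage ticks follow.
; End overlap clears the flag, sets IsBurning true and hides OnFire after a short delay.
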(event `Spawned_Fire`
  (`KismetSystemLibrary.Delay` 10.0)
  (`self.K2_DestroyActor`))

(event `self.CollisionComp.OnComponentBeginOverlap`
  (params (OverlappedComponent :type "PrimitiveComponent Object Reference") (OtherActor :type "Actor Object Reference") (OtherComp :type "PrimitiveComponent Object Reference") (OtherBodyIndex :type Integer) (bFromSweep :type Boolean) (SweepResult :type "HitResult Structure (by ref)"))
  (bind _asbp_mech_character (cast `/Game/Player/BP_MechCharacter` OtherActor))
  (set `self.Player_InRadius` true)
  (`/Game/Player/BP_MechCharacter.InFlame` _asbp_mech_character)
  (`SceneComponent.SetVisibility` (`/Game/Player/BP_MechCharacter.On Fire` _asbp_mech_character) true false)
  (set `/Game/Player/BP_MechCharacter.PlayerHealth` (- (`/Game/Player/BP_MechCharacter.PlayerHealth` _asbp_mech_character) 5.0) _asbp_mech_character :!label _label)
  (`KismetSystemLibrary.Delay` 0.5)
  (if (`self.Player_InRadius`)
    (goto _label)
    (else
      (set `/Game/Player/BP_MechCharacter.PlayerHealth` (- (`/Game/Player/BP_MechCharacter.PlayerHealth` _asbp_mech_character) 5.0) _asbp_mech_character)
      (`KismetSystemLibrary.Delay` 0.5)
      (set `/Game/Player/BP_MechCharacter.PlayerHealth` (- (`/Game/Player/BP_MechCharacter.PlayerHealth` _asbp_mech_character) 5.0) _asbp_mech_character)
      (`KismetSystemLibrary.Delay` 0.5)
      (set `/Game/Player/BP_MechCharacter.PlayerHealth` (- (`/Game/Player/BP_MechCharacter.PlayerHealth` _asbp_mech_character) 5.0) _asbp_mech_character))))

(event `self.CollisionComp.OnComponentEndOverlap`
  (params (OverlappedComponent :type "PrimitiveComponent Object Reference") (OtherActor :type "Actor Object Reference") (OtherComp :type "PrimitiveComponent Object Reference") (OtherBodyIndex :type Integer))
  (bind _asbp_mech_character (cast `/Game/Player/BP_MechCharacter` OtherActor))
  (set `self.Player_InRadius` false)
  (set `/Game/Player/BP_MechCharacter.IsBurning` true _asbp_mech_character)
  (`KismetSystemLibrary.Delay` 1.5)
  (`SceneComponent.SetVisibility` (`/Game/Player/BP_MechCharacter.On Fire` _asbp_mech_character) false false))

(fn `UserConstructionScript`)