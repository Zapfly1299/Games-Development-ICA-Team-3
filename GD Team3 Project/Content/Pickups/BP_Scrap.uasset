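; BP_Scrap is a scrap pickup that pulls itself toward the player's mech and adds one scrap on contact.
; Overlapping the Magnetism component plays the Magnet timeline, which lerps the root from its current transform toward the mech's live capsule location each update, homing on the moving target.
; Overlapping the Box calls ModifyScrap on the mech through a DoOnce, then destroys the pickup after a short delay.
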(event `self.Box.OnComponentBeginOverlap`
  (params (OverlappedComponent :type "PrimitiveComponent Object Reference") (OtherActor :type "Actor Object Reference") (OtherComp :type "PrimitiveComponent Object Reference") (OtherBodyIndex :type Integer) (bFromSweep :type Boolean) (SweepResult :type "HitResult Structure (by ref)"))
  (bind _asbp_mech_character (cast `/Game/Player/BP_MechCharacter` OtherActor))
  (if true
    (`/Engine/EditorBlueprintResources/StandardMacros.DoOnce` false
      (:`Completed`
        (`/Game/Player/BP_MechCharacter.ModifyScrap` _asbp_mech_character 1)
        (`KismetSystemLibrary.Delay` 0.2)
        (`self.K2_DestroyActor`)))))

(event `self.Magnetism.OnComponentBeginOverlap`
  (params (OverlappedComponent :type "PrimitiveComponent Object Reference") (OtherActor :type "Actor Object Reference") (OtherComp :type "PrimitiveComponent Object Reference") (OtherBodyIndex :type Integer) (bFromSweep :type Boolean) (SweepResult :type "HitResult Structure (by ref)"))
  (if (== (`GameplayStatics.GetObjectClass` OtherActor) "/Game/Player/BP_MechCharacter.BP_MechCharacter_C")
    ;[0.0234 0.2344 0] Magnetize to player within radius
    (bind _asbp_mech_character (cast `/Game/Player/BP_MechCharacter` OtherActor))
    (bind (_direction _magnetlerp) (`Timeline|Magnet`)
      (:`Update`
        (`SceneComponent.K2_SetWorldTransform` (`self.DefaultSceneRoot`) (`KismetMathLibrary.TLerp` (`self.GetTransform`) (`KismetMathLibrary.MakeTransform` (`SceneComponent.K2_GetComponentLocation` (`Character.CapsuleComponent` _asbp_mech_character))) _magnetlerp) false false)))))

(fn `UserConstructionScript`)