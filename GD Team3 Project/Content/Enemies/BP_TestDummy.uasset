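; BP_TestDummy is an enemy test dummy with modifiable health and a health bar widget, destroyed when health reaches zero.
; Health starts at max in the construction script, and EnemyHealthModify applies a signed damage or heal amount with clamping.
; BeginPlay passes the actor to WGT_EnemyHealth.
; Each Tick tilts the widget using the camera look-at pitch and roll, with yaw fixed at 180 degrees.
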(event `self.ReceiveBeginPlay`
  (bind _aswgt_enemy_health (cast `/Game/Enemies/WGT_EnemyHealth` (`WidgetComponent.GetUserWidgetObject` (`self.Widget`))))
  (set `/Game/Enemies/WGT_EnemyHealth.EnemyActor` self _aswgt_enemy_health))

(event `self.ReceiveTick`
  (params (DeltaSeconds :type "Float (single-precision)"))
  (`self.RotateHealthBar`))

(fn `EnemyHealthModify`
  (params (`Damage/Heal` :type "Float (double-precision)"))
  (bind _returnvalue (`KismetMathLibrary.FClamp` (+ (`self.EnemyHealth`) `Damage/Heal`) 0.0 (`self.EnemyHealthMax`)))
  (if (<= _returnvalue 0.0)
    (set `self.EnemyHealth` 0.0)
    (`self.K2_DestroyActor`)
    (else
      (set `self.EnemyHealth` _returnvalue))))

(fn `RotateHealthBar`
  (bind _widget (`self.Widget`))
  (bind (_returnvalue_roll _returnvalue_pitch) (`KismetMathLibrary.BreakRotator` (`KismetMathLibrary.FindLookAtRotation` (`SceneComponent.K2_GetComponentLocation` _widget) (`PlayerCameraManager.GetCameraLocation` (`GameplayStatics.GetPlayerCameraManager` 0)))))
  (`SceneComponent.K2_SetWorldRotation` _widget (`KismetMathLibrary.MakeRotator` _returnvalue_roll _returnvalue_pitch 180.0) false false))

(fn `UserConstructionScript`
  (set `self.EnemyHealth` (`self.EnemyHealthMax`)))