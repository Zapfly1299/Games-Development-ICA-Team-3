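; BP_TestEnemy1 is a test enemy with health and a widget health display that references it.
; Construction sets health to maximum; AnyDamage adds the damage value to health with clamping, so only negative values hurt, and destroys the actor at zero.
; Each tick tilts the widget toward the player camera using look-at pitch and roll, with yaw fixed rather than fully billboarded.
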(event `self.ReceiveBeginPlay`
  (bind _aswgt_enemy_health_2 (cast `/Game/Enemies/WGT_EnemyHealth2` (`WidgetComponent.GetUserWidgetObject` (`self.Widget`))))
  (set `/Game/Enemies/WGT_EnemyHealth2.EnemyObject` self _aswgt_enemy_health_2))

(event `self.ReceiveAnyDamage`
  (params (Damage :type "Float (single-precision)") (DamageType :type "DamageType Object Reference") (InstigatedBy :type "Controller Object Reference") (DamageCauser :type "Actor Object Reference"))
  (bind _returnvalue (`KismetMathLibrary.FClamp` (+ (`self.EnemyHealth`) Damage) 0.0 (`self.EnemyHealthMax`)))
  (if (<= _returnvalue 0.0)
    (set `self.EnemyHealth` 0.0)
    (`self.K2_DestroyActor`)
    (else
      (set `self.EnemyHealth` _returnvalue))))

(event `self.ReceiveTick`
  (params (DeltaSeconds :type "Float (single-precision)"))
  (bind _widget (`self.Widget`))
  (bind (_returnvalue_roll _returnvalue_pitch) (`KismetMathLibrary.BreakRotator` (`KismetMathLibrary.FindLookAtRotation` (`SceneComponent.K2_GetComponentLocation` _widget) (`PlayerCameraManager.GetCameraLocation` (`GameplayStatics.GetPlayerCameraManager` 0)))))
  (`SceneComponent.K2_SetWorldRotation` _widget (`KismetMathLibrary.MakeRotator` _returnvalue_roll _returnvalue_pitch 180.0) false false))

(fn `UserConstructionScript`
  (set `self.EnemyHealth` (`self.EnemyHealthMax`)))