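; Level controller that periodically beams enemies in near the player and across a bounding box, tightening both timers once shortly after start.
; PlayArea overlaps track tagged enemies for max-count checks.
; Near spawns use random navigable points; global spawns re-roll points until a sphere trace finds clear space.
; BeamInEnemy plays a sped-up particle effect and spawns a random type, weighted toward the third by clamping.
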(event `self.PlayArea.OnComponentBeginOverlap`
  (params (OverlappedComponent :type "PrimitiveComponent Object Reference") (OtherActor :type "Actor Object Reference") (OtherComp :type "PrimitiveComponent Object Reference") (OtherBodyIndex :type Integer) (bFromSweep :type Boolean) (SweepResult :type "HitResult Structure (by ref)"))
  ;[0.09255 0.3687 1] Keep a list of enemies in the PlayArea as they come and go
  (if (`self.ActorHasTag` OtherActor "Enemy")
    (`KismetArrayLibrary.Array_Add` (`self.EnemiesInPlayArea`) OtherActor)))

(event `self.PlayArea.OnComponentEndOverlap`
  (params (OverlappedComponent :type "PrimitiveComponent Object Reference") (OtherActor :type "Actor Object Reference") (OtherComp :type "PrimitiveComponent Object Reference") (OtherBodyIndex :type Integer))
  ;[0.09255 0.3687 1] Keep a list of enemies in the PlayArea as they come and go
  (if (`self.ActorHasTag` OtherActor "Enemy")
    (`KismetArrayLibrary.Array_RemoveItem` (`self.EnemiesInPlayArea`) OtherActor)))

(event `self.ReceiveBeginPlay`
  (`KismetSystemLibrary.Delay` 4.0)
  (`self.GlobalSpawn`)
  (`self.SpawnEnemiesNearPlayer`)
  (bind _returnvalue (`KismetSystemLibrary.K2_SetTimerDelegate` (delegate `SpawnEnemiesNearPlayer`) 10.0 true))
  (bind _returnvalue_2 (`KismetSystemLibrary.K2_SetTimerDelegate` (delegate `GlobalSpawn`) 15.0 true))
  ;[1 1 1] After 20 seconds, reset spawn event timers but 2 seconds shorter
  (`KismetSystemLibrary.Delay` 21.0)
  (`KismetSystemLibrary.K2_ClearAndInvalidateTimerHandle` _returnvalue_2)
  (`KismetSystemLibrary.K2_ClearAndInvalidateTimerHandle` _returnvalue)
  (`KismetSystemLibrary.K2_SetTimerDelegate` (delegate `SpawnEnemiesNearPlayer`) 8.0 true)
  (`KismetSystemLibrary.K2_SetTimerDelegate` (delegate `GlobalSpawn`) 12.0 true))

(event `SpawnEnemiesNearPlayer`
  ;[1 1 1] Spawn enemies near player
  (for _ (range (+ (`self.SpawnNearNo`) 1))
    (if (< (`KismetArrayLibrary.Array_Length` (`self.EnemiesInPlayArea`)) (`self.MaxEnemies`))
      (bind _output_get (set `self.NearSpawnTargetPoint` (`NavigationSystemV1.K2_GetRandomLocationInNavigableRadius` (`self.K2_GetActorLocation` (`GameplayStatics.GetPlayerCharacter` 0)) 900.0 null null)))
      (`self.BeamInEnemy` _output_get))))

(event `GlobalSpawn`
  ;[1 1 1] Spawn enemies globally
  (for _ (range 1 (+ (`self.SpawnGlobalNo`) 1))
    (if (< (`KismetArrayLibrary.Array_Length` (`self.EnemiesInPlayArea`)) (`self.MaxEnemies`))
      (bind _output_get (set `self.GlobalSpawnTargetPoint` (`KismetMathLibrary.RandomPointInBoundingBox` (`self.K2_GetActorLocation`) (`self.GlobalSpawnBoxExtents`)) :!label _label))
      (bind (_outhit _returnvalue) (`KismetSystemLibrary.SphereTraceSingleForObjects` _output_get _output_get 100.0 (`|MakeArray` "ObjectTypeQuery1" "ObjectTypeQuery2" "ObjectTypeQuery3" "ObjectTypeQuery4" "ObjectTypeQuery6" :!type "EObjectTypeQuery Enum") false (`self.TheFloor`) "Persistent" true (struct :`R` 1.0 :`A` 1.0) (struct :`G` 1.0 :`A` 1.0) 100.0))
      (if _returnvalue
        (goto _label)
        (else
          (`self.BeamInEnemy` (`self.GlobalSpawnTargetPoint`)))))))

(fn `BeamInEnemy`
  (params (Location :type "Vector Structure"))
  (bind _returnvalue (`GameplayStatics.SpawnEmitterAtLocation` "/Game/VFX_Toolkit_V1/ParticleSystems/356Days/Par_BeamIn.Par_BeamIn" Location (struct) (0.5 0.5 1.0)))
  (set `ParticleSystemComponent.CustomTimeDilation` 3.0 _returnvalue)
  (`|SpawnActorFromClass` (`|GetArrayItem` (`self.EnemyTypes`) (`KismetMathLibrary.Clamp` (`KismetMathLibrary.RandomIntegerInRange` 0 5) 0 2)) (`KismetMathLibrary.MakeTransform` Location) "Undefined" "OverrideRootScale" null null))

(fn `UserConstructionScript`)