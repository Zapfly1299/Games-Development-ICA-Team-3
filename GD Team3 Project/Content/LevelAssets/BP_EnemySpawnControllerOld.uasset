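; Enemy spawn controller actor that spawns one AI enemy at a random point inside a box-shaped spawn area when play begins.
; BeginPlay draws a temporary debug box for the area, then spawns the pawn with its behavior tree and a fire particle effect at the chosen point.
; PlayArea overlap events add and remove actors tagged Enemy in EnemiesInPlayArea, which nothing else in this graph reads.
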(event `self.ReceiveBeginPlay`
  (bind _spawnareadimensions (`self.SpawnAreaDimensions`))
  (bind _returnvalue (`SceneComponent.K2_GetComponentLocation` (`self.SpawnAreaCentre`)))
  (`KismetSystemLibrary.DrawDebugBox` _returnvalue _spawnareadimensions (struct :`R` 1.0 :`B` 0.025346 :`A` 1.0) (struct) 10.0)
  (bind _output_get (set `self.EnemySpawnPoint` (`KismetMathLibrary.RandomPointInBoundingBox` _returnvalue _spawnareadimensions)))
  (`AIBlueprintHelperLibrary.SpawnAIFromClass` "/Game/AI/Enemy_AI.Enemy_AI_C" "/Game/AI/BT_AI.BT_AI" _output_get)
  (`GameplayStatics.SpawnEmitterAtLocation` "/Game/StarterContent/Particles/P_Fire.P_Fire" _output_get))

(event `self.PlayArea.OnComponentBeginOverlap`
  (params (OverlappedComponent :type "PrimitiveComponent Object Reference") (OtherActor :type "Actor Object Reference") (OtherComp :type "PrimitiveComponent Object Reference") (OtherBodyIndex :type Integer) (bFromSweep :type Boolean) (SweepResult :type "HitResult Structure (by ref)"))
  (if (`self.ActorHasTag` OtherActor "Enemy")
    (`KismetArrayLibrary.Array_Add` (`self.EnemiesInPlayArea`) OtherActor)))

(event `self.PlayArea.OnComponentEndOverlap`
  (params (OverlappedComponent :type "PrimitiveComponent Object Reference") (OtherActor :type "Actor Object Reference") (OtherComp :type "PrimitiveComponent Object Reference") (OtherBodyIndex :type Integer))
  (if (`self.ActorHasTag` OtherActor "Enemy")
    (`KismetArrayLibrary.Array_RemoveItem` (`self.EnemiesInPlayArea`) OtherActor)))

(fn `UserConstructionScript`)