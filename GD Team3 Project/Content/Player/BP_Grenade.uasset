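; BP_Grenade is a player grenade actor that explodes either when its fuse timer runs out or when an enemy touches it.
; BeginPlay waits for GrenadeTimer, while an overlap on Sphere1 with any actor tagged Enemy detonates it early.
; Explode spawns the explosion particle at the Sphere location, applies full radial damage there, then destroys the actor.
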(event `self.ReceiveBeginPlay`
  (`KismetSystemLibrary.Delay` (`self.GrenadeTimer`))
  (`self.Explode`))

(event `self.Sphere1.OnComponentBeginOverlap`
  (params (OverlappedComponent :type "PrimitiveComponent Object Reference") (OtherActor :type "Actor Object Reference") (OtherComp :type "PrimitiveComponent Object Reference") (OtherBodyIndex :type Integer) (bFromSweep :type Boolean) (SweepResult :type "HitResult Structure (by ref)"))
  (if (`self.ActorHasTag` OtherActor "Enemy")
    (`self.Explode`)))

(fn `Explode`
  (bind _returnvalue (`SceneComponent.K2_GetComponentLocation` (`self.Sphere`)))
  (`GameplayStatics.SpawnEmitterAtLocation` "/Game/StarterContent/Particles/P_Explosion.P_Explosion" _returnvalue (struct) (1.5 1.5 1.5))
  (`GameplayStatics.ApplyRadialDamage` :`BaseDamage` 30.0 :`Origin` _returnvalue :`DamageRadius` 200.0 :`DamageCauser` self :`InstigatedByController` null :`bDoFullDamage` true)
  (`self.K2_DestroyActor`))

(fn `UserConstructionScript`)