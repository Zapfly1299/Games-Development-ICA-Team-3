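; Saw blade projectile that ricochets between enemies, damaging those it hits, and destroys itself after a short lifetime.
; Overlapping an Enemy or StopBullets actor triggers a pawn sphere trace, ignoring the player and last hit enemy, to find the nearest Enemy.
; It turns toward that target and resets its velocity, then applies delayed damage to the last hit enemy.
; Without a target, it applies the damage and destroys itself.
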(event `self.ReceiveBeginPlay`
  (`KismetSystemLibrary.Delay` 2.0)
  (`self.K2_DestroyActor`))

(event `self.Sphere.OnComponentBeginOverlap`
  (params (OverlappedComponent :type "PrimitiveComponent Object Reference") (OtherActor :type "Actor Object Reference") (OtherComp :type "PrimitiveComponent Object Reference") (OtherBodyIndex :type Integer) (bFromSweep :type Boolean) (SweepResult :type "HitResult Structure (by ref)"))
  ;[0.1812 0.4342 1] If you hit an object tagged StopBullets, empty LastHitEnemy
  (if (`self.ActorHasTag` OtherActor "StopBullets")
    (set `self.LastHitEnemy` null)
    ;[1 1 1] Find enemies in boucne range, then find the nearest enemy
    (bind _enemiesinbouncerange (`self.FindEnemiesInBounceRange` (`self.LastHitEnemy`) :!label _label))
    (bind _nearestenemyactor (`self.FindNearestEnemy` _enemiesinbouncerange))
    (if (`KismetSystemLibrary.IsValid` _nearestenemyactor)
      ;[1 1 1] If there's a vaid bounce target, rotate towards it and set velocity in that direction, then deal damage to the last hit enemy
      (`self.K2_SetActorRotation` (`KismetMathLibrary.FindLookAtRotation` (`self.K2_GetActorLocation`) (`self.K2_GetActorLocation` _nearestenemyactor)))
      (`ProjectileMovementComponent.SetVelocityInLocalSpace` (`self.ProjectileMovement`) (1000.0 0.0 0.0))
      (`KismetSystemLibrary.Delay` 0.2)
      (`GameplayStatics.ApplyDamage` (`self.LastHitEnemy`) 20.0)
      (else
        ;[1 1 1] If there's no valid bounce target, deal damage to the last hit actor then destroy self
        (`KismetSystemLibrary.PrintString` "nearestEnemyActor is not valid!")
        (`KismetSystemLibrary.Delay` 0.2)
        (`GameplayStatics.ApplyDamage` (`self.LastHitEnemy`) 20.0)
        (`self.K2_DestroyActor`)))
    (else
      ;[0.1812 0.4342 1] If you hit an actor tagged Enemy, set it as LastHitEnemy
      (if (`self.ActorHasTag` OtherActor "Enemy")
        (set `self.LastHitEnemy` OtherActor)
        (goto _label)))))

(fn `FindEnemiesInBounceRange`
  (params (LastHitActor :type "Actor Object Reference"))
  (returns (EnemiesInBounceRange :type "Array of Actor Object Reference"))
  (bind _returnvalue (`self.K2_GetActorLocation`))
  ;[1 1 1] SphereTrace for every pawn in 500 units, return hit result
  (bind (_outhits _returnvalue_2) (`KismetSystemLibrary.SphereTraceMultiForObjects` _returnvalue _returnvalue 500.0 (`|MakeArray` "ObjectTypeQuery3" :!type "EObjectTypeQuery Enum") false (`|MakeArray` LastHitActor (`GameplayStatics.GetPlayerCharacter` 0) :!type "Actor Object Reference")))
  (if _returnvalue_2
    ;[1 1 1] For each pawn in range, if it has the Enemy tag add it to the EnemiesInRangeArray
    (for _array_element _outhits
      (bind (_bblockinghit _binitialoverlap _time _distance _location _impactpoint _normal _impactnormal _physmat _hitactor) (`GameplayStatics.BreakHitResult` _array_element))
      (if (`self.ActorHasTag` _hitactor "Enemy")
        (`KismetArrayLibrary.Array_Add` (`self.EnemiesInRange`) _hitactor)))
    (return (`self.EnemiesInRange`))
    (else
      (`KismetSystemLibrary.PrintString` "SphereTrace returned no valid pawns")
      (return))))

(fn `FindNearestEnemy`
  (params (EnemiesInBounceRange :type "Array of Actor Object Reference"))
  (returns (NearestEnemyActor :type "Actor Object Reference"))
  (if (> (`KismetArrayLibrary.Array_Length` EnemiesInBounceRange) 0)
    (for _array_element EnemiesInBounceRange
      (bind _returnvalue (`self.GetDistanceTo` _array_element))
      (if (> (`self.NearestEnemyDistance`) _returnvalue)
        (set `self.NearestEnemyDistance` _returnvalue)
        (set `self.NearestEnemy` _array_element)))
    (`KismetArrayLibrary.Array_Clear` (`self.EnemiesInRange`))
    (return (`self.NearestEnemy`))
    (else
      (`KismetSystemLibrary.PrintString` "EnemiesInBounceRange array is empty!")
      (return null))))

(fn `UserConstructionScript`)