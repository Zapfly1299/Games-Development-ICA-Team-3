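; BP_PlayerBullet is the player's projectile actor, which damages enemies and destroys itself on impact or after a short lifetime.
; Its Sphere overlap checks for StopBullets, via either a gameplay tag message or an actor tag, and spawns a small explosion with sound before destroying the bullet.
; Otherwise, actors tagged Enemy take fixed damage and get a larger explosion effect, while other overlaps are ignored.
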(event `self.ReceiveBeginPlay`
  ;[0.1812 0.4342 1] If you hit an object tagged StopBullets, destroy self
  (`KismetSystemLibrary.Delay` 2.0)
  (`self.K2_DestroyActor` :!label _label))

(event `self.Sphere.OnComponentBeginOverlap`
  (params (OverlappedComponent :type "PrimitiveComponent Object Reference") (OtherActor :type "Actor Object Reference") (OtherComp :type "PrimitiveComponent Object Reference") (OtherBodyIndex :type Integer) (bFromSweep :type Boolean) (SweepResult :type "HitResult Structure (by ref)"))
  (bind _returnvalue (`self.K2_GetActorLocation`))
  (bind _returnvalue_2 (`self.K2_GetActorLocation`))
  ;[0.1812 0.4342 1] If you hit an object tagged StopBullets, destroy self
  (bind _returnvalue_3 (message `GameplayTagAssetInterface.HasMatchingGameplayTag` OtherActor (struct :`TagName` "StopBullets")))
  (if (or _returnvalue_3 (`self.ActorHasTag` OtherActor "StopBullets"))
    (`GameplayStatics.SpawnEmitterAtLocation` "/Game/StarterContent/Particles/P_Explosion.P_Explosion" _returnvalue_2 (struct) (0.1 0.1 0.1))
    (`GameplayStatics.PlaySoundAtLocation` "/Game/StarterContent/Audio/Explosion_Cue.Explosion_Cue" _returnvalue_2 (struct) 0.1 1.0 0.0 null null null)
    (goto _label)
    (else
      ;[0.1812 0.4342 1] If you hit an actor tagged Enemy apply damage
      (if (`self.ActorHasTag` OtherActor "Enemy")
        (`GameplayStatics.ApplyDamage` OtherActor 10.0)
        (`GameplayStatics.SpawnEmitterAtLocation` "/Game/StarterContent/Particles/P_Explosion.P_Explosion" _returnvalue (struct) (0.2 0.2 0.2))
        (`GameplayStatics.PlaySoundAtLocation` "/Game/StarterContent/Audio/Explosion_Cue.Explosion_Cue" _returnvalue (struct) 0.1 1.0 0.0 null null null)
        (`self.K2_DestroyActor`)))))

(fn `UserConstructionScript`)