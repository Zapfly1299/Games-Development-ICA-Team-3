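; BP_HomingMissile is a player homing missile projectile that explodes on enemies and expires after three seconds.
; A HomingRadius overlap with an Enemy sets the homing target to OverlappedComponent (the radius itself, not the enemy), then destroys the radius.
; Collision with an Enemy sphere-traces Pawns, applying explosion damage and destroying the missile inside the hit loop.
; MissileHoming is never called; its Homing search keeps the farthest enemy despite its "Closest" naming.
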(event `self.ReceiveBeginPlay`
  (`KismetSystemLibrary.Delay` 3.0)
  (`self.K2_DestroyActor`))

(event `self.HomingRadius.OnComponentBeginOverlap`
  (params (OverlappedComponent :type "PrimitiveComponent Object Reference") (OtherActor :type "Actor Object Reference") (OtherComp :type "PrimitiveComponent Object Reference") (OtherBodyIndex :type Integer) (bFromSweep :type Boolean) (SweepResult :type "HitResult Structure (by ref)"))
  (if (`self.ActorHasTag` OtherActor "Enemy")
    (set `ProjectileMovementComponent.HomingTargetComponent` OverlappedComponent (`self.ProjectileMovement`))
    (`ActorComponent.K2_DestroyComponent` (`self.HomingRadius`))))

(event `MissileHoming`
  (bind _projectilemovement (`self.ProjectileMovement`))
  (bind _selectedtarget (`self.Homing`))
  (set `ProjectileMovementComponent.HomingTargetComponent` _selectedtarget _projectilemovement)
  (set `ProjectileMovementComponent.bIsHomingProjectile` true _projectilemovement)
  (set `MovementComponent.Velocity` (0.0 0.0 0.0) _projectilemovement))

(event `self.Collision.OnComponentBeginOverlap`
  (params (OverlappedComponent :type "PrimitiveComponent Object Reference") (OtherActor :type "Actor Object Reference") (OtherComp :type "PrimitiveComponent Object Reference") (OtherBodyIndex :type Integer) (bFromSweep :type Boolean) (SweepResult :type "HitResult Structure (by ref)"))
  (bind _returnvalue (`SceneComponent.K2_GetComponentLocation` (`self.Collision`)))
  (if (`self.ActorHasTag` OtherActor "Enemy")
    (`/Engine/EditorBlueprintResources/StandardMacros.DoOnce` false
      (:`Completed`
        (bind _outhits (`KismetSystemLibrary.SphereTraceMultiForObjects` :`Start` _returnvalue :`End` _returnvalue :`Radius` (`self.ExplosionRadius`) :`ObjectTypes` (`|MakeArray` "ObjectTypeQuery3" :!type "EObjectTypeQuery Enum") :`DrawDebugType` "ForDuration"))
        (for _array_element _outhits
          (`GameplayStatics.ApplyDamage` (`.HitActor` (`GameplayStatics.BreakHitResult` _array_element)) (`self.ExplosionDamage`))
          (`self.K2_DestroyActor`))))))

(fn `Homing`
  (returns (SelectedTarget :type "SceneComponent Object Reference"))
  (locals (ClosestDistance :type "Float (double-precision)") (ClosestTarget :type "Actor Object Reference"))
  (bind _outactors (`GameplayStatics.GetAllActorsWithTag` "Enemy"))
  (for _array_element _outactors
    (bind _returnvalue (`KismetMathLibrary.VSize` (- (`self.K2_GetActorLocation`) (`SceneComponent.K2_GetComponentLocation` (`Actor.RootComponent` _array_element)))))
    (if (> _returnvalue (`local.ClosestDistance`))
      (set `local.ClosestDistance` _returnvalue)
      (set `local.ClosestTarget` _array_element)))
  (return (`Actor.RootComponent` (`local.ClosestTarget`))))

(fn `UserConstructionScript`)