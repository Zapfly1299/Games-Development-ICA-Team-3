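; Grenade projectile that bounces a limited number of times, then explodes to damage nearby pawns.
; Each bounce decrements a counter; a bounce at zero, or overlap with an Enemy-tagged actor, triggers a one-time explosion.
; The explosion runs a sphere trace for Pawn objects with debug drawing, applies damage per hit and destroys the grenade inside that loop, or directly when nothing is hit.
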(event `self.ProjectileMovement.OnProjectileBounce`
  (params (ImpactResult :type "HitResult Structure (by ref)") (ImpactVelocity :type "Vector Structure (by ref)"))
  (bind _bounces (`self.Bounces`))
  (bind _returnvalue (`SceneComponent.K2_GetComponentLocation` (`self.Collision`)))
  (if (> _bounces 0)
    (set `self.Bounces` (- _bounces 1))
    (else
      (`/Engine/EditorBlueprintResources/StandardMacros.DoOnce` false :!label _label
        (:`Completed`
          (bind (_outhits _returnvalue_2) (`KismetSystemLibrary.SphereTraceMultiForObjects` :`Start` _returnvalue :`End` _returnvalue :`Radius` (`self.ExplosionRadius`) :`ObjectTypes` (`|MakeArray` "ObjectTypeQuery3" :!type "EObjectTypeQuery Enum") :`DrawDebugType` "ForDuration"))
          (if _returnvalue_2
            (for _array_element _outhits
              (`GameplayStatics.ApplyDamage` (`.HitActor` (`GameplayStatics.BreakHitResult` _array_element)) (`self.GrenadeDamage`))
              (`self.K2_DestroyActor` :!label _label_2))
            (else
              (goto _label_2))))))))

(event `self.Collision.OnComponentBeginOverlap`
  (params (OverlappedComponent :type "PrimitiveComponent Object Reference") (OtherActor :type "Actor Object Reference") (OtherComp :type "PrimitiveComponent Object Reference") (OtherBodyIndex :type Integer) (bFromSweep :type Boolean) (SweepResult :type "HitResult Structure (by ref)"))
  (if (`self.ActorHasTag` OtherActor "Enemy")
    (goto _label)))

(fn `UserConstructionScript`)