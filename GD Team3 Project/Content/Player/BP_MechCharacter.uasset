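; Player mech character for a twin-stick shooter, handling movement, aiming, weapons, survival resources and game over.
; Held fire picks the rifle or an ammo-limited alt weapon, including a timeline-charged, line-trace railgun cancelled through a retriggerable delay.
; A looping timer drains energy, with temporary overdrive trading faster drain for quicker rifle fire.
; Shields reduce damage, held repair converts scrap to health, and zero health or energy opens GameOver.
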(event `InputAxis|FireForward`
  (params (AxisValue :type "Float (single-precision)"))
  ;[0.1812 0.4342 1] Find look direction from Fire inputs (look rotation is handled in the anim blueprint)
  (if (> (+ (`KismetMathLibrary.Abs` AxisValue) (`KismetMathLibrary.Abs` (stale `InputAxis|FireRight` AxisValue))) 0.0) :!label _label
    (set `self.NewLookRotation` (`KismetMathLibrary.MakeRotator` 0.0 0.0 (`KismetMathLibrary.GetYawPitchFromVector` (`KismetMathLibrary.MakeVector` (* AxisValue -1.0) (* (stale `InputAxis|FireRight` AxisValue) -1.0)))))
    (if (`self.FireHeld`)
      (if (`self.AltFireOn`)
        (switch `name` (`self.CurrentAltWeapon`)
          (:`Default`
            ;[0.1812 0.4342 1] Shoot Rifle
            (if (`self.CanFire`) :!label _label_2
              (`self.RifleShoot`)
              (set `self.CanFire` false)
              (`KismetSystemLibrary.Delay` (`self.RifleShootCooldown`))
              (set `self.CanFire` true)))
          (:`Shotgun`
            ;[0.1812 0.4342 1] Shoot Shotgun
            (if (`self.CanFire`)
              (`self.ShotgunShoot`)
              (set `self.CanFire` false)
              ;[0.1812 0.4342 1] Decrement ammo, and if ammo is at or below zero empty the Alt Weapon variable
              (`self.DecrementAltFireAmmo`)
              ;[0.1812 0.4342 1] Update AltFireText UI widget, then reenable shooting after a delay
              (`self.UpdateAltFireText`)
              (`KismetSystemLibrary.Delay` (`self.ShotgunShootCooldown`))
              (set `self.CanFire` true)))
          (:`RocketLauncher`
            ;[0.1812 0.4342 1] Shoot Rocket Launcher
            (if (`self.CanFire`)
              (`self.RocketShoot`)
              (set `self.CanFire` false)
              ;[0.1812 0.4342 1] Decrement ammo
              (`self.DecrementAltFireAmmo`)
              ;[0.1812 0.4342 1] Update AltFireText UI widget, then reenable shooting after a delay
              (`self.UpdateAltFireText`)
              (`KismetSystemLibrary.Delay` (`self.RocketShootCooldown`))
              (set `self.CanFire` true)))
          (:`Railgun`
            ;[0.0234 0.2344 0] james: shoot railgun
            (`|ExecutionSequence`
              (:`then_0`
                (`/Engine/EditorBlueprintResources/StandardMacros.DoOnce` false :!label _label_3
                  (:`Completed`
                    (`SceneComponent.SetHiddenInGame` (`self.RailgunBar`) false false)
                    (bind (_direction _railguncharge) (`Timeline|ChargeTime` :!via `PlayFromStart` :!label _label_4)
                      (:`Update`
                        (bind _output_get (set `self.CastBarCharge` _railguncharge))
                        (if (== _output_get 100.0)
                          (`/Engine/EditorBlueprintResources/StandardMacros.DoOnce` false :!label _label_5
                            (:`Completed`
                              (`self.RailShoot`)
                              ;[0.1812 0.4342 1] Decrement ammo blah blah
                              (`self.DecrementAltFireAmmo`)
                              ;[0.0234 0.2344 0] Reset charge bar and cooldown
                              (`self.UpdateAltFireText`)
                              (set `self.CastBarCharge` 0.0)
                              (`SceneComponent.SetHiddenInGame` (`self.RailgunBar`) true false)
                              (`KismetSystemLibrary.Delay` 1.0)
                              (`self.Reset railgun`)))
                          (else
                            (goto _label_5 :!via `Reset`))))))))
              (:`then_1`
                ;[0.1812 0.4342 1] matt: cancelling the railgun
                (`KismetSystemLibrary.RetriggerableDelay` 0.1)
                (set `self.CastBarCharge` 0.0)
                (`SceneComponent.SetHiddenInGame` (`self.RailgunBar`) true false)
                (`self.Reset railgun`)
                (goto _label_4 :!via `Stop`))))
          (:`SawbladeLauncher`
            ;[0.1812 0.4342 1] Shoot Sawblade launcher
            (if (`self.CanFire`)
              (`self.SawbladeShoot`)
              (set `self.CanFire` false)
              ;[0.1812 0.4342 1] decrement ammo
              (`self.DecrementAltFireAmmo`)
              ;[0.1812 0.4342 1] update ui and start fire cooldown
              (`self.UpdateAltFireText`)
              (`KismetSystemLibrary.Delay` (`self.GrenadeShootCooldown`))
              (set `self.CanFire` true))))
        (else
          (goto _label_2))))))

(event `InputAxis|MoveForward`
  (params (AxisValue :type "Float (single-precision)"))
  ;[0.1812 0.4342 1] Locomotion
  (`self.AddMovementInput` (1.0 0.0 0.0) AxisValue)
  ;[0.1812 0.4342 1] Rotate towards movement vector when there's a move input
  (if (> (+ (`KismetMathLibrary.Abs` AxisValue) (`KismetMathLibrary.Abs` (stale `InputAxis|MoveRight` AxisValue))) 0.0) :!label _label_6
    (`Controller.SetControlRotation` (`self.GetController`) (`KismetMathLibrary.MakeRotator` 0.0 0.0 (`KismetMathLibrary.GetYawPitchFromVector` (`KismetMathLibrary.MakeVector` AxisValue (stale `InputAxis|MoveRight` AxisValue)))))))

(event `InputAxis|FireRight`
  (params (AxisValue :type "Float (single-precision)"))
  ;[0.1812 0.4342 1] Find look direction from Fire inputs (look rotation is handled in the anim blueprint)
  (goto _label))

(event `InputAxis|MoveRight`
  (params (AxisValue :type "Float (single-precision)"))
  ;[0.1812 0.4342 1] Locomotion
  (`self.AddMovementInput` (0.0 1.0 0.0) AxisValue)
  (goto _label_6))

(event `InputAction|AltFire`
  (params (Key :type "Key Structure"))
  ;[0.1812 0.4342 1] Toggle using the AltFire
  (:`Pressed`
    (set `self.AltFireOn` true))
  (:`Released`
    (set `self.AltFireOn` false)))

(event `Reset railgun`
  ;[0.0234 0.2344 0] james: shoot railgun
  (goto _label_3 :!via `Reset`))

(event `OverdriveActivate`
  ;[1 0.4446 0.1392] Overdrive system
  (`self.OverdriveMacro`))

(event `InputAction|HoldToFire`
  (params (Key :type "Key Structure"))
  ;[0.1812 0.4342 1] Toggle whether player is firing
  (:`Pressed`
    (set `self.FireHeld` true))
  (:`Released`
    (set `self.FireHeld` false)))

(event `self.ReceiveBeginPlay`
  ;[0.1812 0.4342 1] Player Energy system
  (`KismetSystemLibrary.K2_SetTimerDelegate` (delegate `SubtractEnergy`) 1.0 true))

(event `SubtractEnergy`
  ;[0.1812 0.4342 1] Player Energy system
  (bind _output_get (set `self.PlayerEnergy` (`KismetMathLibrary.FClamp` (- (`self.PlayerEnergy`) (`self.EnergyDrainRate`)) 0.0 (`self.PlayerEnergyMax`))))
  ;[0.0234 0.2344 0] James  - Game Over on energy zero
  (if (<= _output_get 0.0)
    (`self.Shutdown`)))

(event `Shutdown`
  ;[0.0234 0.2344 0] James  - Game Over on energy zero
  (`self.DisableInput` null)
  (`SkeletalMeshComponent.PlayAnimation` (`self.Mesh`) "/Game/Default_Sleep.Default_Sleep" false)
  (`KismetSystemLibrary.Delay` 1.0)
  (`GameplayStatics.OpenLevel` "GameOver"))

(event `AddEnergy`
  ;[0.1812 0.4342 1] Player Energy system
  (set `self.PlayerEnergy` (+ (`self.PlayerEnergy`) 10.0)))

(event `self.ReceiveAnyDamage`
  (params (Damage :type "Float (single-precision)") (DamageType :type "DamageType Object Reference") (InstigatedBy :type "Controller Object Reference") (DamageCauser :type "Actor Object Reference"))
  ;[0.1812 0.4342 1] Player health/ take damage
  (if (`self.ShieldActive`)
    (bind _damageout (`self.Shielding` Damage))
    (`self.ModifyHealth` _damageout)
    (else
      (`self.ModifyHealth` Damage))))

(event `InputAction|ScrapRepair`
  (params (Key :type "Key Structure"))
  (bind _charactermovement (`self.CharacterMovement`))
  ;[0.0234 0.2344 0] James - Replenishes health (repairs the mech) while either left face button e.g. X on xbox controller or Q on the keyboard is held
  (:`Pressed`
    (`CharacterMovementComponent.DisableMovement` _charactermovement)
    (bind _returnvalue (`KismetSystemLibrary.K2_SetTimerDelegate` (delegate `RepairMode`) 0.5 true)))
  (:`Released`
    (`CharacterMovementComponent.SetMovementMode` _charactermovement "MOVE_Walking" 0)
    (`KismetSystemLibrary.K2_ClearAndInvalidateTimerHandle` _returnvalue :!label _label_7)))

(event `RepairMode`
  ;[0.0234 0.2344 0] James - Replenishes health (repairs the mech) while either left face button e.g. X on xbox controller or Q on the keyboard is held
  ;;[1 1 1 0.5] Checking if player health is at max and player has any scrap
  (if (or (== (`self.PlayerHealth`) (`self.PlayerHealthMax`)) (< (`self.PlayerScrap`) 1))
    (goto _label_7)
    (else
      ;;[1 1 1 0.5] Inreases player health and depletes scrap count
      (set `self.PlayerHealth` (`KismetMathLibrary.FClamp` (+ (`self.PlayerHealth`) 5.0) 0.0 (`self.PlayerHealthMax`)))
      (`self.ModifyScrap` -1))))

(event `Key|P`
  (params (Key :type "Key Structure"))
  (bind _returnvalue (`GameplayStatics.GetPlayerController` 0))
  ;[0.2396 1 0.2554] Call Pause Menu
  (:`Pressed`
    (`GameplayStatics.SetGamePaused` true)
    (bind _returnvalue_2 (`|CreateWidget` "/Game/Levels/Level_UI/PauseMenu.PauseMenu_C" _returnvalue))
    (`UserWidget.AddToViewport` _returnvalue_2 0)
    (set `PlayerController.bShowMouseCursor` true _returnvalue)
    (`WidgetBlueprintLibrary.SetInputMode_UIOnlyEx` _returnvalue _returnvalue_2)))

(event `IsDead`
  (bind _returnvalue (`SceneComponent.K2_GetComponentLocation` (`self.Mesh`)))
  ;[0.2604 1 0.2772] Player Death
  (`/Engine/EditorBlueprintResources/StandardMacros.DoOnce` false
    (:`Completed`
      (`GameplayStatics.SpawnEmitterAtLocation` "/Game/StarterContent/Particles/P_Explosion.P_Explosion" _returnvalue (struct) (1.5 1.0 1.0))
      (`GameplayStatics.SpawnSoundAtLocation` "/Game/StarterContent/Audio/Explosion_Cue.Explosion_Cue" _returnvalue (struct) 1.0 1.0 0.0 null null)
      (`CharacterMovementComponent.DisableMovement` (`self.CharacterMovement`))
      (`SkeletalMeshComponent.PlayAnimation` (`self.Mesh`) "/Game/Player/Mech/Models/mech_Anim_Hit.mech_Anim_Hit" false)
      (`self.DisableInput` null)
      (`KismetSystemLibrary.Delay` 2.0)
      (`GameplayStatics.OpenLevel` "GameOver"))))

(fn `AddEnergyFunc`
  (bind _output_get (set `self.PlayerEnergy` (+ (`self.PlayerEnergy`) 10.0)))
  (if (> _output_get (`self.PlayerEnergyMax`))
    (set `self.PlayerEnergy` (`self.PlayerEnergyMax`))))

(fn `DecrementAltFireAmmo`
  (`/Engine/EditorBlueprintResources/StandardMacros.DecrementInt` (`self.AltFireAmmo`)
    (:`  `
      (if (<= (`self.AltFireAmmo`) 0)
        (set `self.CurrentAltWeapon` "None"))
      (return))))

(fn `ModifyHealth`
  (params (Damage :type "Float (double-precision)"))
  (bind _output_get (set `self.PlayerHealth` (`KismetMathLibrary.FClamp` (- (`self.PlayerHealth`) Damage) 0.0 (`self.PlayerHealthMax`))))
  (if (<= _output_get 0.0)
    (`self.IsDead`)))

(fn `ModifyScrap`
  (params (ScrapChange :type Integer))
  (set `self.PlayerScrap` (+ ScrapChange (`self.PlayerScrap`)))
  (`self.UpdateScrap`))

(fn `RailShoot`
  (bind _rifleshootarrowleft (`self.RifleShootArrowLeft`))
  (bind _rifleshootarrowright (`self.RifleShootArrowRight`))
  (bind _hittargets (`self.HitTargets`))
  (bind _returnvalue (`SceneComponent.K2_GetComponentLocation` _rifleshootarrowright))
  (bind _returnvalue_2 (`SceneComponent.K2_GetComponentLocation` _rifleshootarrowleft))
  ;[0.0234 0.2344 0] James - Railgun Firing
  (`self.PlayAnimMontage` "/Game/Player/Mech/Models/mech_Anim_ShootBigCanon_A_Montage.mech_Anim_ShootBigCanon_A_Montage" 1.2)
  (`GameplayStatics.PlaySoundAtLocation` "/Game/Player/Mech/Sounds/BigCanon.BigCanon" (`SceneComponent.K2_GetComponentLocation` (`self.CapsuleComponent`)) (struct) 1.0 1.0 0.0 null null null)
  (`|ExecutionSequence`
    (:`then_0`
      ;;[1 1 1 0.5] Trace control
      (bind _outhits (`KismetSystemLibrary.LineTraceMultiForObjects` _returnvalue_2 (+ _returnvalue_2 (* (`KismetMathLibrary.GetForwardVector` (`SceneComponent.K2_GetComponentRotation` _rifleshootarrowleft)) 3000.0)) (`|MakeArray` "ObjectTypeQuery3" :!type "EObjectTypeQuery Enum")))
      ;;[1 1 1 0.5] enemy damage control
      (`KismetArrayLibrary.Array_Append` _hittargets _outhits))
    (:`then_1`
      (bind _outhits_2 (`KismetSystemLibrary.LineTraceMultiForObjects` _returnvalue (+ _returnvalue (* (`KismetMathLibrary.GetForwardVector` (`SceneComponent.K2_GetComponentRotation` _rifleshootarrowright)) 3000.0)) (`|MakeArray` "ObjectTypeQuery3" :!type "EObjectTypeQuery Enum")))
      (`KismetArrayLibrary.Array_Append` _hittargets _outhits_2)
      (for _array_element _hittargets
        (`GameplayStatics.ApplyDamage` (`.HitActor` (`GameplayStatics.BreakHitResult` _array_element)) 50.0))
      (`KismetArrayLibrary.Array_Clear` (`self.HitTargets`)))))

(fn `RifleShoot`
  (bind _returnvalue (`SceneComponent.K2_GetComponentToWorld` (`self.RifleShootArrowRight`)))
  (bind _returnvalue_2 (`SceneComponent.K2_GetComponentToWorld` (`self.RifleShootArrowLeft`)))
  (`self.PlayAnimMontage` "/Game/Player/Mech/Models/mech_Anim_ShootBigCanon_A_Montage.mech_Anim_ShootBigCanon_A_Montage" 1.2)
  (`|SpawnActorFromClass` "/Game/Player/BP_PlayerBullet.BP_PlayerBullet_C" _returnvalue_2 "Undefined" "OverrideRootScale" null null)
  (`|SpawnActorFromClass` "/Game/Player/BP_PlayerBullet.BP_PlayerBullet_C" _returnvalue "Undefined" "OverrideRootScale" null null)
  (`GameplayStatics.SpawnEmitterAtLocation` "/Game/StarterContent/Particles/P_Explosion.P_Explosion" (.location _returnvalue) (.rotation _returnvalue) (0.1 0.1 0.1))
  (`GameplayStatics.SpawnEmitterAtLocation` "/Game/StarterContent/Particles/P_Explosion.P_Explosion" (.location _returnvalue_2) (.rotation _returnvalue_2) (0.1 0.1 0.1))
  (`GameplayStatics.PlaySoundAtLocation` "/Game/Player/PlayerSounds/soundscrate-rifle.soundscrate-rifle" (`self.K2_GetActorLocation`) (struct) 0.5 1.0 0.0 null null null))

(fn `RocketShoot`
  (`|SpawnActorFromClass` "/Game/Player/BP_HomingProjectile.BP_HomingProjectile_C" (`SceneComponent.K2_GetComponentToWorld` (`self.RocketShootArrow`)) "Undefined" "OverrideRootScale" null null))

(fn `SawbladeShoot`
  (bind _rocketshootarrow (`self.RocketShootArrow`))
  ;[0.1812 0.4342 1] Spawn and launch grenade
  (`|SpawnActorFromClass` "/Game/Player/BP_SawBlade.BP_SawBlade_C" (`KismetMathLibrary.MakeTransform` (`SceneComponent.K2_GetComponentLocation` _rocketshootarrow) (`SceneComponent.K2_GetComponentRotation` _rocketshootarrow)) "Undefined" "OverrideRootScale" null null))

(fn `Shielding`
  (params (DamageIn :type "Float (double-precision)"))
  (returns (DamageOut :type "Float (double-precision)"))
  (locals (DamageTaken :type "Float (double-precision)") (CurrentShield :type "Float (double-precision)"))
  (bind _damagetaken (`local.DamageTaken`))
  ;[0.0234 0.2344 0] James - Shielding
  (set `local.DamageTaken` DamageIn)
  (bind _output_get (set `local.CurrentShield` (- (`self.ShieldValue`) DamageIn)))
  (if (<= _output_get 0.0)
    ;;[1 1 1] Handles incoming damage exceeding shielding
    (set `self.ShieldValue` 0.0)
    (set `local.DamageTaken` (`KismetMathLibrary.Conv_IntToDouble` (`KismetMathLibrary.Round` (+ (`local.DamageTaken`) (* (`local.CurrentShield`) (`self.ArmourValue`))))))
    (set `self.ShieldActive` false)
    (else
      ;;[1 1 1] Multiples incoming damage by a decimel to get % reduced then deducts that from damage to be taken.
      (set `self.ShieldValue` (`local.CurrentShield`))
      (set `local.DamageTaken` (`KismetMathLibrary.Conv_IntToDouble` (`KismetMathLibrary.Round` (- _damagetaken (* _damagetaken (`self.ArmourValue`))))))))
  (return (`local.DamageTaken`)))

(fn `ShotgunShoot`
  (`self.PlayAnimMontage` "/Game/Player/Mech/Models/mech_Anim_ShootBigCanon_A_Montage.mech_Anim_ShootBigCanon_A_Montage" 1.2)
  (for (_array_element _array_index) (`SceneComponent.GetChildrenComponents` (`self.Mesh`) false)
    (if (and (>= _array_index 0) (<= _array_index 5))
      (`|SpawnActorFromClass` "/Game/Player/BP_PlayerBullet.BP_PlayerBullet_C" (`SceneComponent.K2_GetComponentToWorld` _array_element) "Undefined" "OverrideRootScale" null null))))

(fn `UserConstructionScript`)